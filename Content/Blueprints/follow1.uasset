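; Actor Blueprint that moves itself along the spline of a Splinepathbp actor found in the level at BeginPlay.
; The MoveObjectT timeline, with play rate set from TimetoComplete, drives a Lerp from full spline length down to zero.
; Each update sets the actor transform using the world location at that distance; a spline rotation lookup exists but is unused.
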(event `self.ReceiveBeginPlay`
  (bind _returnvalue (`GameplayStatics.GetActorOfClass` "/Game/Blueprints/splinepathbp.splinepathbp_C"))
  (set `self.NewVar_1` _returnvalue)
  (`self.moveobject`))

(event `moveobject`
  (`TimelineComponent.SetPlayRate` (`self.Move Object T`) (/ 1.0 (`self.TimetoComplete`)))
  (bind (_direction _move_track) (`Timeline|Move Object T`)
    (:`Update`
      (`self.K2_SetActorTransform` (`KismetMathLibrary.MakeTransform` (`SplineComponent.GetLocationAtDistanceAlongSpline` (`/Game/Blueprints/splinepathbp.Spline` (`self.NewVar_1`)) (`KismetMathLibrary.Lerp` (`SplineComponent.GetSplineLength` (`/Game/Blueprints/splinepathbp.Spline` (`self.NewVar_1`))) 0.0 _move_track) "World"))))))

(fn `UserConstructionScript`)