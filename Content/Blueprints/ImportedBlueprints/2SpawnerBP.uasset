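; An audio-reactive spawner actor that spawns rocks in response to a sound it plays.
; BeginPlay starts the sound and binds its playback-percent event, which converts progress into elapsed seconds.
; Each update reads channel 0 of a precomputed Constant-Q analysis at that time and spawns a Rock_bp at the Arrow's transform for every band above a high threshold.
; The delays in BeginPlay lead to no further actions.
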(event `self.ReceiveBeginPlay`
  (bind _audio (`self.Audio`))
  (bind _mysound (`self.MySound`))
  (`|ExecutionSequence`
    (:`then_0`
      (`AudioComponent.SetSound` _audio _mysound)
      (set `self.Duration` (`SoundBase.Duration` _mysound))
      (add `AudioComponent.OnAudioPlaybackPercent` _audio (delegate `Play Sound`))
      (`AudioComponent.Play` (`self.Audio`) 0.0)
      (`KismetSystemLibrary.Delay` 25.0))
    (:`then_1`
      (`KismetSystemLibrary.Delay` 42.0))))

(event `Play Sound`
  (params (PlayingSoundWave :type "SoundWave Object Reference") (PlaybackPercent :type "Float (single-precision)"))
  (set `self.PlayedTime` (* PlaybackPercent (`self.Duration`)))
  (for _array_element (`ConstantQNRT.GetNormalizedChannelConstantQAtTime` (`self.MySoundNRT`) (`self.PlayedTime`) 0)
    (if (> _array_element 0.91)
      (`|SpawnActorFromClass` "/Game/Blueprints/ImportedBlueprints/rock_bp.rock_bp_C" (`SceneComponent.K2_GetComponentToWorld` (`self.Arrow`)) "AdjustIfPossibleButDontSpawnIfColliding" "MultiplyWithRoot" null null))))

(fn `UserConstructionScript`)